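; Base player controller that sets up per-platform input and toggles the package (inventory) screen.
; On possess, mobile platforms get a simple touch widget, while Windows and other platforms add the mouse-look Enhanced Input mapping context.
; The OpenPackage event calls OpenInventory, which uses a shown flag to hide or create and show the package widget through the base UMG manager.
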(event `self.ReceivePossess`
  (params (PossessedPawn :type "Pawn Object Reference"))
  (switch `string` (`GameplayStatics.GetPlatformName`)
    (:`Default`
      (`EnhancedInputSubsystemInterface.AddMappingContext` (subsystem `EnhancedInputLocalPlayerSubsystem`) "/Game/Input/IMC_MouseLook.IMC_MouseLook" 0 (struct) :!label _label))
    (:`Windows`
      (goto _label))
    (:`Android`
      (bind _returnvalue (`|CreateWidget` "/Game/Input/Touch/UI_TouchSimple.UI_TouchSimple_C" :!label _label_2))
      (`UserWidget.AddToPlayerScreen` _returnvalue 0))
    (:`IOS`
      (goto _label_2))))

(event `self.OpenPackage`
  (`self.OpenInventory`))

(fn `OpenInventory`
  (locals (Package :type "BaseUserWidget Object Reference"))
  (bind _returnvalue (`InventorySystemFuncLib.GetBaseUMGManager` null))
  (bind _returnvalue_2 (`BaseUMGManager.GetUMGWidget` _returnvalue "/Game/UI/WBP_PackageWidget.WBP_PackageWidget_C" -1 true))
  (set `local.Package` _returnvalue_2)
  (`self.bShownPacakage`
    (:`then`
      (bind _returnvalue_3 (`InventorySystemFuncLib.GetBaseUMGManager` null))
      (bind _package (`local.Package`)
        (:`then`
          (`BaseUMGManager.HideUMGWidget` _returnvalue_3 _package))
        (:`else`
          _))
      (set `self.bShownPacakage` false))
    (:`else`
      (bind _returnvalue_4 (`InventorySystemFuncLib.GetBaseUMGManager` null))
      (bind _returnvalue_5 (`BaseUMGManager.CreateUMGWidget` _returnvalue_4 "/Game/UI/WBP_PackageWidget.WBP_PackageWidget_C"))
      (bind _output_get (set `local.Package` _returnvalue_5))
      (`BaseUMGManager.ShowUMGWidget` _returnvalue_4 _output_get 0)
      (set `self.bShownPacakage` true))))

(fn `UserConstructionScript`)